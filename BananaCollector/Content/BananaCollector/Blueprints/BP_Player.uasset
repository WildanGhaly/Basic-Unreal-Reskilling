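; Player pawn for Banana Collector that moves on forward and right axis input without using a movement component's logic.
; A shared Move function adds movement input along the actor's forward or right vector, scaled by MovementSpeed.
; Tick consumes the accumulated vector and applies it, scaled by delta time, as a swept offset.
; That offset is applied in local space, although the input directions are world-space vectors.
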(event EventBeginPlay)

(event Collision|EventActorBeginOverlap
  (params (OtherActor :type Actor%20Object%20Reference)))

(event EventTick
  (params (DeltaSeconds :type Float%20%28single-precision%29))
  (bind _returnvalue (Class|Pawn|ConsumeMovementInputVector))
  (Transformation|AddActorLocalOffset (* _returnvalue DeltaSeconds) true false))

(event Input|AxisEvents|InputAxisMoveForward
  (params (AxisValue :type Float%20%28single-precision%29))
  (CallFunction|Move true AxisValue))

(event Input|AxisEvents|InputAxisMoveRight
  (params (AxisValue :type Float%20%28single-precision%29))
  (CallFunction|Move false AxisValue))

(fn ConstructionScript)

(fn Move
  (params (IsForward :type Boolean) (MoveDirection :type Float%20%28double-precision%29))
  (bind _movementspeed (Variables|Default|GetMovementSpeed))
  (bind _returnvalue (* MoveDirection _movementspeed))
  (if IsForward
    ;[1 1 1] Move Forward
    (Pawn|Input|AddMovementInput (Transformation|GetActorForwardVector) _returnvalue false)
    (else
      ;[1 1 1] Move Right
      (Pawn|Input|AddMovementInput (Transformation|GetActorRightVector) _returnvalue false))))