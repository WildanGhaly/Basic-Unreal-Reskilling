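; BP_Tunnel is a tunnel segment for an endless runner, with a rotating holed wall that kills BP_Player on hit.
; The wall rolls every tick in a direction randomly chosen at BeginPlay.
; When the player overlaps CollisionTrigger, the segment has TunnelSpawner spawn another tunnel, then destroys itself.
; RandomizeWall and RandomizeTunnel vary hole mesh, starting roll and tunnel material, but are not called within this Blueprint.
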(event OnComponentBeginOverlap(CollisionTrigger)
  (params (OverlappedComponent :type Primitive%20Component%20Object%20Reference) (OtherActor :type Actor%20Object%20Reference) (OtherComp :type Primitive%20Component%20Object%20Reference) (OtherBodyIndex :type Integer) (bFromSweep :type Boolean) (SweepResult :type Hit%20Result%20Structure%20%28by%20ref%29))
  (Utilities|Casting|CastToBP_Player OtherActor)
  (Utilities|FlowControl|Sequence
    (:then_0
      (Default|SpawnTunnelatSpawnPoint (Variables|Default|GetTunnelSpawner)))
    (:then_1
      (Actor|DestroyActor))))

(event OnComponentHit(WallMesh)
  (params (HitComponent :type Primitive%20Component%20Object%20Reference) (OtherActor :type Actor%20Object%20Reference) (OtherComp :type Primitive%20Component%20Object%20Reference) (NormalImpulse :type Vector :default "0, 0, 0") (Hit :type Hit%20Result%20Structure%20%28by%20ref%29))
  (bind _asbp_player (Utilities|Casting|CastToBP_Player OtherActor))
  (Default|KillPlayer _asbp_player))

(event EventBeginPlay
  (Variables|Default|SetIsBackward (Math|Random|RandomBool)))

(event EventTick
  (params (DeltaSeconds :type Float%20%28single-precision%29))
  (CallFunction|RotateWall DeltaSeconds))

(fn ConstructionScript)

(fn RotateWall
  (params (DeltaTime :type Float%20%28double-precision%29))
  (bind _rotationspeed (Variables|Default|GetRotationSpeed))
  (bind _wallmesh (Variables|Default|GetWallMesh))
  (bind _returnvalue (* DeltaTime _rotationspeed))
  (if (Variables|Default|GetIsBackward)
    (Transformation|AddLocalRotation _wallmesh (Math|Rotator|MakeRotator _returnvalue 0.0 0.0) false false)
    (else
      (Transformation|AddLocalRotation _wallmesh (Math|Rotator|MakeRotator (* _returnvalue -1.0) 0.0 0.0) false false))))

(fn RandomizeWall
  (bind _wallmesh (Variables|Default|GetWallMesh))
  (Components|StaticMesh|SetStaticMesh _wallmesh (Utilities|Select :Index (Math|Random|RandomIntegerinRange 0 3) :Option%200 "/Game/InfiniteMatrix/Meshes/SM_Hole_01.SM_Hole_01" :Option%201 "/Game/InfiniteMatrix/Meshes/SM_Hole_02.SM_Hole_02" :Option%202 "/Game/InfiniteMatrix/Meshes/SM_Hole_03.SM_Hole_03" :Option%203 "/Game/InfiniteMatrix/Meshes/SM_Hole_04.SM_Hole_04"))
  (Transformation|AddLocalRotation _wallmesh (Math|Rotator|MakeRotator (Math|Random|RandomFloatinRange 0.0 3.6e+02) 0.0 0.0) false false))

(fn RandomizeTunnel
  (Rendering|Material|SetMaterial (Variables|Debug|GetStaticMeshComponent) 0 (Utilities|Select :Index (Math|Random|RandomIntegerinRange 0 3) :Option%200 "/Game/InfiniteMatrix/Materials/MI_Tunnel.MI_Tunnel" :Option%201 "/Game/InfiniteMatrix/Materials/MI_Tunnel_Blue.MI_Tunnel_Blue" :Option%202 "/Game/InfiniteMatrix/Materials/MI_Tunnel_Purple.MI_Tunnel_Purple" :Option%203 "/Game/InfiniteMatrix/Materials/MI_Tunnel_Red.MI_Tunnel_Red")))