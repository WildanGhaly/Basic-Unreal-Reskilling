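; Spawner actor that builds a chain of randomized BP_Tunnel segments for the player in InfiniteMatrix.
; On BeginPlay it destroys any existing tunnels, then spawns three, starting at the player pawn's location when no valid newest tunnel exists.
; Each further segment attaches at the newest tunnel's SpawnLocation component, receives a reference back to the spawner, and randomizes its wall and tunnel.
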(event EventBeginPlay
  (CallFunction|SpawnTunnelInnit))

(event Collision|EventActorBeginOverlap
  (params (OtherActor :type Actor%20Object%20Reference)))

(event EventTick
  (params (DeltaSeconds :type Float%20%28single-precision%29)))

(fn ConstructionScript)

(fn SpawnTunnel
  (params (SpawnLocation :type Vector))
  (bind _returnvalue (Game|SpawnActorfromClass "/Game/InfiniteMatrix/Blueprints/BP_Tunnel.BP_Tunnel_C" (Math|Transform|MakeTransform SpawnLocation "0, 0, 0" "1.000000,1.000000,1.000000") "Undefined" "MultiplyWithRoot" 0 0))
  (bind _output_get (Variables|Default|SetNewestTunnel _returnvalue))
  (Variables|/Game/InfiniteMatrix/Blueprints/BP_Tunnel.BP_Tunnel_C|SetTunnelSpawner _output_get self)
  (Default|RandomizeWall _output_get)
  (Default|RandomizeTunnel _output_get))

(fn SpawnTunnelatSpawnPoint
  (CallFunction|SpawnTunnel (Transformation|GetWorldLocation (Variables|/Game/InfiniteMatrix/Blueprints/BP_Tunnel.BP_Tunnel_C|GetSpawnLocation (Variables|Default|GetNewestTunnel)))))

(fn SpawnTunnelInnit
  (Utilities|FlowControl|Sequence
    (:then_0
      (CallFunction|DestroyTunnel))
    (:then_1
      (CallFunction|SpawnNTunnel 3))))

(fn DestroyTunnel
  (bind _outactors (Actor|GetAllActorsOfClass "/Game/InfiniteMatrix/Blueprints/BP_Tunnel.BP_Tunnel_C"))
  (for _array_element _outactors
    (Actor|DestroyActor _array_element)))

(fn SpawnNTunnel
  (params (Number%20of%20Tunnel :type Integer))
  (for _index (range 1 Number%20of%20Tunnel)
    (Utilities|IsValid (Variables|Default|GetNewestTunnel)
      (:Is%20Valid
        (CallFunction|SpawnTunnelatSpawnPoint))
      (:Is%20Not%20Valid
        (CallFunction|SpawnTunnel (Transformation|GetActorLocation (Game|Player|GetPlayerPawn 0)))))))